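; Game mode that loads city weather records from a database and lists them in a UI-only main menu widget.
; On BeginPlay it opens the database, parses cities JSON, waits a fixed two-second delay, then reads the data back.
; It then creates WBP_Main and passes each record's temperature, description, wind and time to the widget's list.
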(event EventBeginPlay
  (Class|MainGameModeBase|OpenDatabase)
  (Class|MainGameModeBase|ParseCitiesJson)
  (Utilities|FlowControl|Delay 2.0)
  (Class|MainGameModeBase|GetDatafromDatabase)
  (bind _returnvalue (UserInterface|CreateWidget "/Game/Blueprints/WBP_Main.WBP_Main_C"))
  (bind _output_get (Variables|Default|SetMainWidget _returnvalue))
  (UserInterface|Viewport|AddtoViewport _output_get 0)
  (Input|SetInputModeUIOnly (Game|GetPlayerController 0) 0 "DoNotLock")
  (CallFunction|AddCitiestoList))

(event EventTick
  (params (DeltaSeconds :type Float%20%28single-precision%29)))

(fn ConstructionScript)

(fn AddCitiestoList
  (for _array_element (Variables|Default|GetCityInfoFromDB)
    (Default|AddDatatoList (Variables|Default|GetMainWidget) (Utilities|Struct|MakeS_CitiesInfo (.City (Utilities|Struct|BreakDataFromDB _array_element)) (.TemperatureEstimated (Utilities|Struct|BreakDataFromDB _array_element)) (.TemperatureFeel (Utilities|Struct|BreakDataFromDB _array_element)) (.WeatherDesription (Utilities|Struct|BreakDataFromDB _array_element)) (.WindSpeed (Utilities|Struct|BreakDataFromDB _array_element)) (.DateTime (Utilities|Struct|BreakDataFromDB _array_element))))))